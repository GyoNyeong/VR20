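; BP_Timer is an actor that shows an elapsed-time clock as minutes:seconds on a TextRender component.
; While GoTimer is true, Tick accumulates delta seconds scaled by 30, so the clock runs at thirty times normal speed.
; The total is split by division and modulo 60, and FlaotToStr00 floors and zero-pads each part.
; An older minute-counter draft is left unconnected, and Test only prints a debug string.
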(event `self.ReceiveTick`
  (params (DeltaSeconds :type "Float (single-precision)"))
  ;[1 1 1 1 12] Delta Second 를 전부 누적하면 초단위 공정한 시간 값을 얻을 수 있다.
  (if (`self.GoTimer`)
    (bind _output_get (set `self.TotalDeltaSeconds` (+ (* DeltaSeconds 30.0) (`self.TotalDeltaSeconds`))))
    (`TextRenderComponent.K2_SetText` (`self.TextRender`) (`KismetTextLibrary.Conv_StringToText` (`KismetStringLibrary.Concat_StrStr` (`self.FlaotToStr00` (/ _output_get 60.0)) ":" (`self.FlaotToStr00` (mod _output_get 60.0)))))))

(fn `FlaotToStr00`
  (params (Number :type "Float (double-precision)"))
  (returns (Str00 :type String))
  (bind _returnvalue (`KismetMathLibrary.FFloor` Number))
  (bind _returnvalue_2 (`KismetStringLibrary.Conv_IntToString` _returnvalue))
  (if (< _returnvalue 10)
    (return (`KismetStringLibrary.Concat_StrStr` "0" _returnvalue_2))
    (else
      (return _returnvalue_2))))

(fn `Test`
  (`KismetSystemLibrary.PrintString` "Hello"))

(fn `UserConstructionScript`)