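; BP_LeftRight is an actor that shuttles back and forth along world X around its starting position.
; On the first Tick, a DoOnce records the location and sets bounds 100 units either side.
; Each Tick then applies a fixed, frame-rate-dependent offset and flips the Right flag once a bound is passed.
; An alternative Timeline-driven movement remains in the graph but never runs.
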(event `self.ReceiveBeginPlay`)

(event `self.ReceiveTick`
  (params (DeltaSeconds :type "Float (single-precision)"))
  (bind _returnvalue_x (`KismetMathLibrary.BreakVector` (`self.K2_GetActorLocation`)))
  (bind _returnvalue_x_2 (`KismetMathLibrary.BreakVector` (`self.K2_GetActorLocation`)))
  (`|ExecutionSequence`
    (:`then_0`
      (`/Engine/EditorBlueprintResources/StandardMacros.DoOnce` false
        (:`Completed`
          (bind _output_get (set `self.Cur` (`self.K2_GetActorLocation`)))
          (set `self.Max` (+ (.x _output_get) 100.0))
          (set `self.Min` (- (.x _output_get) 100.0)))))
    (:`then_1`
      (if (`self.Right`)
        (`self.K2_AddActorWorldOffset` (2.0 0.0 0.0))
        (if (> _returnvalue_x_2 (`self.Max`))
          (set `self.Right` false))
        (else
          (`self.K2_AddActorWorldOffset` (-2.0 0.0 0.0))
          (if (< _returnvalue_x (`self.Min`))
            (set `self.Right` true)))))))

(fn `UserConstructionScript`)