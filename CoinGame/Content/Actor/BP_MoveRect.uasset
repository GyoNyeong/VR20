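; BP_MoveRect is an actor that moves its Cube component around a rectangular path between 0 and 100 on relative X and Y.
; Each Tick switches on the Move direction, steps X or Y by one and sets the cube's relative location.
; Reaching an edge switches Move to the next direction, cycling Right, Up, Left, Down.
; The step ignores delta time, so speed depends on frame rate.
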(event `self.ReceiveTick`
  (params (DeltaSeconds :type "Float (single-precision)"))
  (bind (_relativelocation_x _relativelocation_y) (`KismetMathLibrary.BreakVector` (`SceneComponent.RelativeLocation` (`self.Cube`))))
  (bind _relativelocation_x_2 (`KismetMathLibrary.BreakVector` (`SceneComponent.RelativeLocation` (`self.Cube`))))
  (bind (_relativelocation_x_3 _relativelocation_y_2) (`KismetMathLibrary.BreakVector` (`SceneComponent.RelativeLocation` (`self.Cube`))))
  (bind _relativelocation_x_4 (`KismetMathLibrary.BreakVector` (`SceneComponent.RelativeLocation` (`self.Cube`))))
  (switch `/Game/Actor/EM_MoveType` (`self.move`)
    (:`NewEnumerator0`
      (bind _result (`/Engine/EditorBlueprintResources/StandardMacros.DecrementFloat` (`self.X`))
        (:`  `
          (`SceneComponent.K2_SetRelativeLocation` (`self.Cube`) (`KismetMathLibrary.MakeVector` _result (`self.Y`)) false false)
          (if (<= _relativelocation_x_4 0.0)
            (set `self.move` "NewEnumerator3")))))
    (:`NewEnumerator1`
      (bind _result_2 (`/Engine/EditorBlueprintResources/StandardMacros.IncrementFloat` (`self.X`))
        (:`  `
          (`SceneComponent.K2_SetRelativeLocation` (`self.Cube`) (`KismetMathLibrary.MakeVector` _result_2 (`self.Y`)) false false)
          (if (>= _relativelocation_x_2 100.0)
            (set `self.move` "NewEnumerator2")))))
    (:`NewEnumerator2`
      (bind _result_3 (`/Engine/EditorBlueprintResources/StandardMacros.IncrementFloat` (`self.Y`))
        (:`  `
          (`SceneComponent.K2_SetRelativeLocation` (`self.Cube`) (`KismetMathLibrary.MakeVector` (`self.X`) _result_3) false false)
          (if (>= _relativelocation_y_2 100.0)
            (set `self.move` "NewEnumerator0")))))
    (:`NewEnumerator3`
      (bind _result_4 (`/Engine/EditorBlueprintResources/StandardMacros.DecrementFloat` (`self.Y`))
        (:`  `
          (`SceneComponent.K2_SetRelativeLocation` (`self.Cube`) (`KismetMathLibrary.MakeVector` (`self.X`) _result_4) false false)
          (if (<= _relativelocation_y 0.0)
            (set `self.move` "NewEnumerator1")))))))

(fn `UserConstructionScript`)