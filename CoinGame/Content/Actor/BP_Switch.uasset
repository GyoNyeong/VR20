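; BP_Switch is an overlap switch that activates linked level actors while the third-person character stands in it and deactivates them on exit.
; Begin and end overlap pass true or false to helper functions that set Start, IsMove and GoTimer across the Move, Moverect and Timer arrays.
; Spawners are played or stopped directly in a loop, leaving the PlaySpawner helper unused.
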(event `self.ReceiveActorBeginOverlap`
  (params (OtherActor :type "Actor Object Reference"))
  (cast `/Game/ThirdPerson/Blueprints/BP_ThirdPersonCharacter` OtherActor)
  (`self.LeftLight` (`self.move`) true)
  (`self.Rect` (`self.moverect`) true)
  (`self.TimerSet` (`self.Timer`) true)
  (for _array_element (`self.Spawner`)
    (`/Game/Actor/BP_Spawner.Play` _array_element)))

(event `self.ReceiveActorEndOverlap`
  (params (OtherActor :type "Actor Object Reference"))
  (cast `/Game/ThirdPerson/Blueprints/BP_ThirdPersonCharacter` OtherActor)
  (`self.LeftLight` (`self.move`))
  (`self.Rect` (`self.moverect`))
  (`self.TimerSet` (`self.Timer`))
  (for _array_element (`self.Spawner`)
    (`/Game/Actor/BP_Spawner.Stop` _array_element)))

(fn `LeftLight`
  (params (NewParam :type "Array of /Game/Actor/BP_LeftRight Object Reference") (NewParam1 :type Boolean))
  (for _array_element NewParam
    (set `/Game/Actor/BP_LeftRight.start` NewParam1 _array_element)))

(fn `PlaySpawner`
  (params (NewParam :type "Array of /Game/Actor/BP_Spawner Object Reference") (NewParam1 :type Boolean))
  (for _array_element NewParam
    (set `/Game/Actor/BP_Spawner.DoPlay` NewParam1 _array_element)))

(fn `Rect`
  (params (NewParam :type "Array of /Game/Actor/BP_MoveRect Object Reference") (NewParam1 :type Boolean))
  (for _array_element NewParam
    (set `/Game/Actor/BP_MoveRect.Is Move?` NewParam1 _array_element)))

(fn `TimerSet`
  (params (NewParam :type "Array of /Game/Actor/BP_Timer Object Reference") (NewParam1 :type Boolean))
  (for _array_element NewParam
    (set `/Game/Actor/BP_Timer.GoTimer` NewParam1 _array_element)))

(fn `UserConstructionScript`)