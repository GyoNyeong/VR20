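; Behavior tree task that stores the player character as the AI's target in the blackboard.
; On AI execute, it gets player character 0 and, if valid, writes it to the blackboard key selected by TargetChr and finishes successfully.
; If no valid player character exists, the task finishes as failed and leaves the key untouched.
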(event `self.ReceiveExecuteAI`
  (params (OwnerController :type "AIController Object Reference") (ControlledPawn :type "Pawn Object Reference"))
  (bind _returnvalue (`GameplayStatics.GetPlayerCharacter` 0))
  (`/Engine/EditorBlueprintResources/StandardMacros.IsValid` _returnvalue
    (:`Is Valid`
      (`BTFunctionLibrary.SetBlackboardValueAsObject` (`self.TargetChr`) _returnvalue)
      (`self.FinishExecute` true))
    (:`Is Not Valid`
      (`self.FinishExecute` false))))